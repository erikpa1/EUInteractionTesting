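; SC_ClickComponent is an interactable scene component that so far mostly holds debug scaffolding for avatar click interaction.
; On BeginPlay it prints each direct child component's name and, if AutoDeactivate is set, disables the owning actor's collision inside that loop.
; Its AvatarInteracted event only prints the same child names, ignoring the Avatar argument.
; A SetCollisionEnabled(NoCollision) call is left unconnected and never runs.
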(event EventBeginPlay
  (for _array_element (Components|GetChildrenComponents self false)
    (Development|PrintString (Utilities|GetDisplayName _array_element))
    (if (Variables|Default|GetAutoDeactivate)
      (Collision|SetActorEnableCollision (Components|GetOwner) false))))

(event EventTick
  (params (DeltaSeconds :type Float%20%28single-precision%29)))

(event Custom|AvatarInteractedEvent_Event
  (params (Avatar :type BP%20Avatar%20Object%20Reference))
  (for _array_element (Components|GetChildrenComponents false)
    (Development|PrintString (Utilities|GetDisplayName _array_element))))