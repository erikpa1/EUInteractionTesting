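; Base Blueprint for mouse-interactable objects, providing shared avatar interaction events and hover highlight helpers.
; The interacted event only prints a debug string, while the hovered and unhovered events are empty.
; Separate hover and unhover functions toggle custom depth rendering on OutlinableObject when it is valid, which suggests a post-process outline.
; The hover events in this graph do not call those functions.
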(event Custom|AvatarUnhovered_Event
  (params (Avatar :type BP%20Avatar%20Object%20Reference)))

(event Custom|AvatarInteracted_Event
  (params (Avatar :type BP%20Avatar%20Object%20Reference))
  (Development|PrintString "Parent interacted"))

(event Custom|AvatarHovered_Event
  (params (Avatar :type BP%20Avatar%20Object%20Reference)))

(event EventBeginPlay)

(event Collision|EventActorBeginOverlap
  (params (OtherActor :type Actor%20Object%20Reference)))

(event EventTick
  (params (DeltaSeconds :type Float%20%28single-precision%29)))

(fn ConstructionScript)

(fn FnHover
  (bind _outlinableobject (Variables|Default|GetOutlinableObject))
  (if (Utilities|IsValid _outlinableobject)
    (Rendering|SetRenderCustomDepth _outlinableobject true)))

(fn FnUnhover
  (bind _outlinableobject (Variables|Default|GetOutlinableObject))
  (if (Utilities|IsValid _outlinableobject)
    (Rendering|SetRenderCustomDepth _outlinableobject false)))