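; ExampleItem is a sample interactable item from the CharacterApi that hides itself when an avatar interacts with it.
; On BeginPlay it casts its InteractionZone child actor to ClickZone and binds to that zone's AvatarInteracted event.
; The handler prints a debug message and turns off DefaultSceneRoot visibility, propagating to child components, without destroying the actor.
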(event Custom|_AvatarInteracted_Event
  (Development|PrintString "Item going to hide")
  (Rendering|SetVisibility (Variables|Default|GetDefaultSceneRoot) false true))

(event EventBeginPlay
  (|CallParentFunction)
  (bind _asclick_zone (Utilities|Casting|CastToClickZone (Variables|/Script/Engine.ChildActorComponent|GetChildActor (Variables|Default|GetInteractionZone))))
  (EventDispatchers|BindEventtoAvatarInteracted _asclick_zone (delegate Custom|_AvatarInteracted_Event)))

(event Collision|EventActorBeginOverlap
  (params (OtherActor :type Actor%20Object%20Reference))
  (|CallParentFunction OtherActor) ; This node is disabled and will not be called.\nDrag off pins to build functionality.
)

(event EventTick
  (params (DeltaSeconds :type Float%20%28single-precision%29))
  (|CallParentFunction DeltaSeconds) ; This node is disabled and will not be called.\nDrag off pins to build functionality.
)

(fn ConstructionScript
  (|CallParentFunction))