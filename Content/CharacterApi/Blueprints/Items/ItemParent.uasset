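; ItemParent is an item Blueprint, named as a parent class, for objects an avatar picks up into its inventory.
; Both the InteractionPressed event and the AvatarInteracted function hide the root component and pass the item itself to the avatar's inventory widget via AddItem, leaving the actor undestroyed.
; The event also prints a debug message and hides only the root, while the function propagates hiding to child components.
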(event Custom|InteractionPressed_Event
  (params (Avatar :type BP%20Avatar%20Object%20Reference))
  (Development|PrintString "ItemParentClicked" true true "(R=0.047835,G=1.000000,B=0.402959,A=1.000000)")
  (Rendering|SetVisibility (Variables|Default|GetDefaultSceneRoot) false false)
  (Default|AddItem (Variables|/Game/CharacterApi/Blueprints/BP_Avatar.BP_Avatar_C|GetInventory_WID Avatar) self))

(event EventBeginPlay)

(event Collision|EventActorBeginOverlap
  (params (OtherActor :type Actor%20Object%20Reference)))

(event EventTick
  (params (DeltaSeconds :type Float%20%28single-precision%29)))

(fn ConstructionScript)

(fn AvatarInteracted
  (params (Avatar :type BP%20Avatar%20Object%20Reference))
  (Rendering|SetVisibility (Variables|Default|GetDefaultSceneRoot) false true)
  (Default|AddItem (Variables|/Game/CharacterApi/Blueprints/BP_Avatar.BP_Avatar_C|GetInventory_WID Avatar) self))